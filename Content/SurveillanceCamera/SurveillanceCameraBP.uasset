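; Surveillance camera that signals its detection state through a decal colour, shocks a detected player and raises an alarm.
; A cone overlap tracks the tagged player and toggles the HUD's in-range display.
; State changes recolour a dynamic decal material green, yellow or red; red shows an electric beam and spawns a burst on the player.
; Raising the alarm dispatches it, hides the beam and updates the HUD.
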(event OnComponentBeginOverlap(SurveillanceCone)
  (params (OverlappedComponent :type Primitive%20Component%20Object%20Reference) (OtherActor :type Actor%20Object%20Reference) (OtherComp :type Primitive%20Component%20Object%20Reference) (OtherBodyIndex :type Integer) (bFromSweep :type Boolean) (SweepResult :type Hit%20Result%20Structure%20%28by%20ref%29))
  (if (Actor|ActorHasTag OtherActor "Player")
    (Variables|Default|SetdetectedPlayer OtherActor)
    (bind _asmeta_ui (Utilities|Casting|CastToMeta_UI (HUD|GetHUD (Game|GetPlayerController 0))))
    (Default|ShowinCameraRange _asmeta_ui)))

(event OnComponentEndOverlap(SurveillanceCone)
  (params (OverlappedComponent :type Primitive%20Component%20Object%20Reference) (OtherActor :type Actor%20Object%20Reference) (OtherComp :type Primitive%20Component%20Object%20Reference) (OtherBodyIndex :type Integer))
  (if (Actor|ActorHasTag OtherActor "Player")
    (Variables|Default|SetdetectedPlayer 0)
    (bind _asmeta_ui (Utilities|Casting|CastToMeta_UI (HUD|GetHUD (Game|GetPlayerController 0))))
    (Default|HideMetaUI _asmeta_ui)))

(event EventBeginPlay
  (bind _returnvalue (Rendering|Material|CreateDynamicMaterialInstance "/Game/SurveillanceCamera/AreaMaterial.AreaMaterial" "None" "None" :!class /Script/Engine.KismetMaterialLibrary))
  (bind _output_get (Variables|Default|SetDecalMaterial _returnvalue))
  (Rendering|Components|Decal|SetDecalMaterial (Variables|Default|GetDecal) _output_get)
  (Rendering|Material|SetVectorParameterValue (Variables|Default|GetDecalMaterial) "Color" "(R=0.163822,G=1.000000,B=0.000000,A=1.000000)" :!class /Script/Engine.MaterialInstanceDynamic)
  (Rendering|SetVisibility (Variables|Default|GetElectricShock) false false))

(event Collision|EventActorBeginOverlap
  (params (OtherActor :type Actor%20Object%20Reference)))

(event EventTick
  (params (DeltaSeconds :type Float%20%28single-precision%29)))

(event EventOnRaiseAlarm
  (Development|PrintString "Alarm")
  (Default|CallAlarmDispatch)
  (CallFunction|EndShockPlayer)
  (bind _asmeta_ui (Utilities|Casting|CastToMeta_UI (HUD|GetHUD (Game|GetPlayerController 0))))
  (Default|ShowAlarm _asmeta_ui))

(event EventOnStateChange
  (params (newState :type CameraState%20Enum :default "kSeeking"))
  (switch Utilities|FlowControl|Switch|SwitchonCameraState newState
    (:kSeeking
      (Rendering|Material|SetVectorParameterValue (Variables|Default|GetDecalMaterial) "Color" "(R=0.163822,G=1.000000,B=0.000000,A=1.000000)" :!class /Script/Engine.MaterialInstanceDynamic)
      (CallFunction|EndShockPlayer))
    (:kAnalyzing
      (Rendering|Material|SetVectorParameterValue (Variables|Default|GetDecalMaterial) "Color" "(R=1.000000,G=0.956041,B=0.000000,A=1.000000)" :!class /Script/Engine.MaterialInstanceDynamic))
    (:kAlarm
      (Rendering|Material|SetVectorParameterValue (Variables|Default|GetDecalMaterial) "Color" "(R=1.000000,G=0.017204,B=0.000000,A=1.000000)" :!class /Script/Engine.MaterialInstanceDynamic)
      (CallFunction|ShockPlayer))))

(fn ConstructionScript)

(fn ShockPlayer
  (Utilities|FlowControl|Sequence
    (:then_0
      ;[1 1 1] ElectricShock From camera to player
      (Effects|Components|ParticleSystem|SetActorParameter (Variables|Default|GetElectricShock) "EndPoint" (Variables|Default|GetdetectedPlayer))
      (Rendering|SetVisibility (Variables|Default|GetElectricShock) true false))
    (:then_1
      ;[1 1 1] ShockBurst in player
      (bind _returnvalue (Game|SpawnActorfromClass "/Game/ElectricShock/ElectricShockBurst_BP.ElectricShockBurst_BP_C" (Transformation|GetActorTransform (Variables|Default|GetdetectedPlayer)) "Undefined" "MultiplyWithRoot" 0 0))
      (Effects|Components|ParticleSystem|SetActorParameter (Variables|/Game/ElectricShock/ElectricShockBurst_BP.ElectricShockBurst_BP_C|GetEectricityBurst _returnvalue) "Center" (Variables|Default|GetdetectedPlayer)))))

(fn EndShockPlayer
  (Rendering|SetVisibility (Variables|Default|GetElectricShock) false false))